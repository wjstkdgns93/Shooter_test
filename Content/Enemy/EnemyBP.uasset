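; Enemy actor that damages the player character on overlap and reports its death to the game mode.
; Beginning overlap with CharacterBP deals damage immediately, then a looping timer repeats it until the overlap ends.
; DecreaseHP subtracts from Hp and, at zero or below, lowers the GameModeBP enemy count, raises the score and destroys the actor.
; BeginPlay sets Hp to zero, so any positive damage kills it.
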(event `self.ReceiveBeginPlay`
  (set `self.hp` 0.0)
  (bind _asgame_mode_bp (cast `/Game/GameModeBP` (`GameplayStatics.GetGameMode`)))
  (set `self.GameMode` _asgame_mode_bp))

(event `self.ReceiveActorBeginOverlap`
  (params (OtherActor :type "Actor Object Reference"))
  (bind _ascharacter_bp (cast `/Game/Character/CharacterBP` OtherActor))
  (`self.DecreaseCHarHP`)
  (`KismetSystemLibrary.K2_SetTimer` null "DecreaseCHarHP" 0.2 true))

(event `DecreaseCHarHP`
  (`/Game/Interface/DamageInterface.DecreaseHP` (stale `self.ReceiveActorBeginOverlap` _ascharacter_bp) 20.0))

(event `self.ReceiveActorEndOverlap`
  (params (OtherActor :type "Actor Object Reference"))
  (cast `/Game/Character/CharacterBP` OtherActor)
  (`KismetSystemLibrary.K2_ClearTimer` null "DecreaseCHarHP"))

(event `/Game/Interface/DamageInterface.DecreaseHP`
  (params (amount :type "Float (single-precision)"))
  (bind _gamemode (`self.GameMode`))
  (bind _output_get (set `self.hp` (- (`self.hp`) amount)))
  (if (<= _output_get 0.0)
    (`/Game/GameModeBP.Decrease Enemies` _gamemode)
    (`/Game/GameModeBP.Increase Score` _gamemode)
    (`self.K2_DestroyActor`)))

(fn `UserConstructionScript`)