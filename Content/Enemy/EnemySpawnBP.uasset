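; Enemy spawner actor that fills the level with AI enemies at random points inside its Spawn box volume.
; On BeginPlay it caches GameModeBP and starts a looping half-second timer calling SpawnEnemy.
; SpawnEnemy spawns EnemyBP only while the game mode's enemy count is within a small cap, then increments that count.
; A duplicate Spawning event and an unconnected timer setup chain are left unused.
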(event `self.ReceiveBeginPlay`
  (bind _asgame_mode_bp (cast `/Game/GameModeBP` (`GameplayStatics.GetGameMode`)))
  (set `self.GameMode` _asgame_mode_bp)
  (`KismetSystemLibrary.K2_SetTimer` null "SpawnEnemy" 0.5 true))

(event `SpawnEnemy`
  (bind _gamemode (`self.GameMode`))
  (bind _spawn (`self.Spawn`))
  (if (<= (`/Game/GameModeBP.NumberEnemies` _gamemode) 10)
    (`AIBlueprintHelperLibrary.SpawnAIFromClass` "/Game/Enemy/EnemyBP.EnemyBP_C" null (`KismetMathLibrary.RandomPointInBoundingBox` (`SceneComponent.K2_GetComponentLocation` _spawn) (`BoxComponent.GetScaledBoxExtent` _spawn)))
    (`/Game/GameModeBP.Increase Enemies` _gamemode)))

(event `Spawning`
  (bind _gamemode (`self.GameMode`))
  (bind _spawn (`self.Spawn`))
  (if (<= (`/Game/GameModeBP.NumberEnemies` _gamemode) 10)
    (`AIBlueprintHelperLibrary.SpawnAIFromClass` "/Game/Enemy/EnemyBP.EnemyBP_C" null (`KismetMathLibrary.RandomPointInBoundingBox` (`SceneComponent.K2_GetComponentLocation` _spawn) (`BoxComponent.GetScaledBoxExtent` _spawn)))
    (`/Game/GameModeBP.Increase Enemies` _gamemode)))

(fn `UserConstructionScript`)